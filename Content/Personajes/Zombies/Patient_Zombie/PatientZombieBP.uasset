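; Patient zombie enemy Blueprint that chases the player character on sight and plays a melee attack animation on reaching it.
; Pawn sensing starts an AI MoveTo that reissues itself through a short retriggerable delay, skipped while a montage plays; arrival triggers the attack montage.
; Tick updates the health widget's progress bar from Health and yaws the widget component to face the player camera.
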(event `self.PawnSensing.OnSeePawn`
  (params (Pawn :type "Pawn Object Reference"))
  (bind _returnvalue (`AnimInstance.IsAnyMontagePlaying` (`SkeletalMeshComponent.GetAnimInstance` (`self.Mesh`))))
  ;[1 1 1] Inteligencia Artificial
  (bind _asue_4asp_character (cast `/Game/AnimStarterPack/Ue4ASP_Character` Pawn :!label _label))
  (if (not _returnvalue)
    (`|AIMoveTo` self (0.0 0.0 0.0) _asue_4asp_character 10.0
      (:`then`
        (`KismetSystemLibrary.RetriggerableDelay` 0.1)
        (goto _label))
      (:`OnSuccess`
        (if (not _returnvalue)
          (`|PlayMontage` (`self.Mesh`) "/Game/Personajes/Zombies/ZombieAnimations/ZombiePatient_Attack.ZombiePatient_Attack"))))))

(event `self.ReceiveTick`
  (params (DeltaSeconds :type "Float (single-precision)"))
  ;[1 1 1] Salud_Enemigo
  (bind _assalud_patient (cast `/Game/Personajes/Zombies/Patient_Zombie/Salud_Patient` (`WidgetComponent.GetUserWidgetObject` (`self.Salud`))))
  (`ProgressBar.SetPercent` (`/Game/Personajes/Zombies/Patient_Zombie/Salud_Patient.ProgressBar_38` _assalud_patient) (/ (`self.Health`) 200.0))
  (`SceneComponent.K2_SetWorldRotation` (`self.Salud`) (`KismetMathLibrary.MakeRotator` 0.0 0.0 (.yaw (`KismetMathLibrary.FindLookAtRotation` (`SceneComponent.K2_GetComponentLocation` (`self.Salud`)) (`self.K2_GetActorLocation` (`GameplayStatics.GetPlayerCameraManager` 0))))) false false))

(fn `UserConstructionScript`
  (`parent.UserConstructionScript`))